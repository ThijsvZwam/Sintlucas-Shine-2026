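; BP_WaveManager runs enemy waves, spawning BP_Enemy actors round-robin across every TargetPoint in the level.
; StartWave increments the requested count and decrements MaxWaves, then SpawnNextEnemy re-calls itself after a delay, counting each enemy alive post-delay.
; Once MaxWaves is exhausted, it triggers a cutscene instead of spawning.
; EnemyKilled completes the player's quest objective when none remain alive and passes the result to BP_MusicManager for a phase change.
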(event Custom|StartWave
  (params (EnemyAmount :type Integer))
  (bind _result (Math|Integer|DecrementInt (Variables|Default|GetMaxWaves))
    (:%20%20
      (Variables|Default|SetMaxWaves _result)
      (Variables|Default|SetSpawnIndex 0)
      (bind _result_2 (Math|Integer|IncrementInt EnemyAmount)
        (:%20%20
          (bind _output_get (Variables|Default|SetEnemiesToSpawnThisWave _result_2))
          (bind _output_get_2 (Variables|Default|SetEnemiesRemainingInWave _output_get))
          (bind _result_3 (Math|Integer|IncrementInt (Variables|Default|GetWaveNumber))
            (:%20%20
              (Variables|Default|SetWaveNumber _result_3)
              (Variables|Default|SetEnemiesAlive 0)
              (CallFunction|SpawnNextEnemy))))))))

(event Custom|SpawnNextEnemy
  (if (<= (Variables|Default|GetMaxWaves) 0)
    (if (<= (Variables|Default|GetMaxWaves) 0)
      (Default|CallStartCustcene))
    (elif (> (Variables|Default|GetEnemiesRemainingInWave) 0)
      (Game|SpawnActorfromClass "/Game/FightingSystem/Enemies/BP_Enemy.BP_Enemy_C" (Math|Conversions|ToTransform(Vector) (Math|Vector|MakeVector (.X (Math|Vector|BreakVector (Transformation|GetActorLocation (Utilities|Array|Get(acopy) (Variables|Default|GetSpawnPoints) (Math|Integer|%(Integer) (Variables|Default|GetSpawnIndex) (Utilities|Array|Length (Variables|Default|GetSpawnPoints))))))) (.Y (Math|Vector|BreakVector (Transformation|GetActorLocation (Utilities|Array|Get(acopy) (Variables|Default|GetSpawnPoints) (Math|Integer|%(Integer) (Variables|Default|GetSpawnIndex) (Utilities|Array|Length (Variables|Default|GetSpawnPoints))))))) (.Z (Math|Vector|BreakVector (Transformation|GetActorLocation (Utilities|Array|Get(acopy) (Variables|Default|GetSpawnPoints) (Math|Integer|%(Integer) (Variables|Default|GetSpawnIndex) (Utilities|Array|Length (Variables|Default|GetSpawnPoints))))))))) "Undefined" "MultiplyWithRoot" 0 0)
      (bind _result (Math|Integer|IncrementInt (Variables|Default|GetSpawnIndex))
        (:%20%20
          (Variables|Default|SetSpawnIndex _result)
          (bind _result_2 (Math|Integer|DecrementInt (Variables|Default|GetEnemiesRemainingInWave))
            (:%20%20
              (Variables|Default|SetEnemiesRemainingInWave _result_2)
              (Utilities|FlowControl|Delay (Variables|Default|GetSpawnDelay))
              (bind _result_3 (Math|Integer|IncrementInt (Variables|Default|GetEnemiesAlive))
                (:%20%20
                  (bind _output_get (Variables|Default|SetEnemiesAlive _result_3))
                  (Development|PrintString (Utilities|String|ToString(Integer) _output_get))
                  (CallFunction|SpawnNextEnemy))))))))))

(event Custom|EnemyKilled
  (bind _result (Math|Integer|DecrementInt (Variables|Default|GetEnemiesAlive))
    (:%20%20
      (bind _output_get (Variables|Default|SetEnemiesAlive _result))
      (if (<= (Variables|Default|GetEnemiesAlive) 0)
        (bind _asbp_third_person_character (Utilities|Casting|CastToBP_ThirdPersonCharacter (Game|GetPlayerCharacter 0)))
        (bind _musicphase (Default|CompleteObjective (Variables|/Game/ThirdPerson/Blueprints/BP_ThirdPersonCharacter.BP_ThirdPersonCharacter_C|GetQuestManagerRef _asbp_third_person_character)))
        (bind _returnvalue (Actor|GetActorOfClass "/Game/Music/BP_MusicManager.BP_MusicManager_C"))
        (Default|RequestPhaseChange _returnvalue _musicphase)))))

(event EventBeginPlay
  (bind _outactors (Actor|GetAllActorsOfClass "/Script/Engine.TargetPoint"))
  (Variables|Default|SetSpawnPoints _outactors))

(event Collision|EventActorBeginOverlap
  (params (OtherActor :type Actor%20Object%20Reference)))

(event EventTick
  (params (DeltaSeconds :type Float%20%28single-precision%29)))

(fn ConstructionScript)