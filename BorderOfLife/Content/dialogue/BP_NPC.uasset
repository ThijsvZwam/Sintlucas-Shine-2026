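; BP_NPC is a talkable NPC that steps through dialogue lines and then starts a quest.
; Each Talk call advances an index into the Dialogue and Name arrays, showing the current entry in a reused WBP_Dialogue widget with a bounce animation.
; While talking, player look, movement and attack are disabled.
; After the last line it removes the widget, restores controls, resets the index, calls StartQuest on the player's QuestManagerRef and hides ArrowW.
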(event EventTalk
  (bind _returnvalue (Game|GetPlayerController 0))
  (bind _returnvalue_2 (Game|GetPlayerController 0))
  (Math|Integer|IncrementInt (Variables|Default|GettalkIndex)
    (:%20%20
      (if (< (Variables|Default|GettalkIndex) (Utilities|Array|Length (Variables|Default|GetDialogue)))
        (Input|SetIgnoreLookInput _returnvalue true)
        (Input|SetIgnoreMoveInput _returnvalue true)
        (bind _asbp_third_person_character (Utilities|Casting|CastToBP_ThirdPersonCharacter (Game|GetPlayerCharacter 0)))
        (Variables|/Game/ThirdPerson/Blueprints/BP_ThirdPersonCharacter.BP_ThirdPersonCharacter_C|SetbCanAttack _asbp_third_person_character false)
        (Variables|Default|GetUI
          (:then
            _)
          (:else
            (bind _returnvalue_3 (UserInterface|CreateWidget "/Game/dialogue/WBP_Dialogue.WBP_Dialogue_C" (Game|GetPlayerController 0)))
            (bind _output_get (Variables|Default|SetUI _returnvalue_3))
            (UserInterface|Viewport|AddtoViewport _output_get 0)))
        (Variables|/Script/UMG.TextBlock|SetText (Variables|/Game/dialogue/WBP_Dialogue.WBP_Dialogue_C|GetTalkText (Variables|Default|GetUI)) (Utilities|Text|ToText(String) (Utilities|Array|Get(acopy) (Variables|Default|GetDialogue) (Variables|Default|GettalkIndex))))
        (Variables|/Script/UMG.TextBlock|SetText (Variables|/Game/dialogue/WBP_Dialogue.WBP_Dialogue_C|GetNameText (Variables|Default|GetUI)) (Utilities|Text|ToText(String) (Utilities|Array|Get(acopy) (Variables|Default|GetName) (Variables|Default|GettalkIndex))))
        (UserInterface|Animation|PlayAnimation (Variables|Default|GetUI) (Variables|/Game/dialogue/WBP_Dialogue.WBP_Dialogue_C|GetBounce (Variables|Default|GetUI)) 0.0 1 "Forward" 1.0 false)
        (else
          (Class|Controller|ResetIgnoreInputFlags (Game|GetPlayerController 0))
          (Widget|RemovefromParent (Variables|Default|GetUI))
          (Variables|Default|SetUI 0)
          (Variables|Default|SettalkIndex -1)
          (bind _asbp_third_person_character_2 (Utilities|Casting|CastToBP_ThirdPersonCharacter (Game|GetPlayerCharacter 0)))
          (Variables|/Game/ThirdPerson/Blueprints/BP_ThirdPersonCharacter.BP_ThirdPersonCharacter_C|SetIsTalking _asbp_third_person_character_2 false)
          (Variables|/Game/ThirdPerson/Blueprints/BP_ThirdPersonCharacter.BP_ThirdPersonCharacter_C|SetbCanAttack _asbp_third_person_character_2 true)
          (Variables|/Script/Engine.PlayerController|SetbShowMouseCursor _returnvalue_2 false)
          (Input|SetInputModeGameOnly _returnvalue_2 false)
          (bind _asbp_third_person_character_3 (Utilities|Casting|CastToBP_ThirdPersonCharacter (Game|GetPlayerCharacter 0)))
          (Default|StartQuest (Variables|/Game/ThirdPerson/Blueprints/BP_ThirdPersonCharacter.BP_ThirdPersonCharacter_C|GetQuestManagerRef _asbp_third_person_character_3))
          (Rendering|SetVisibility (Variables|Default|GetArrowW) false false))))))

(fn ConstructionScript)