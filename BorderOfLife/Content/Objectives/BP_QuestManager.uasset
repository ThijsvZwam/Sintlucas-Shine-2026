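; Quest manager actor that holds an ordered objective list, with two hardcoded quest starters: a gate quest and a kill-enemies quest.
; Each starter appends objectives, resets the current index and refreshes the main UI through the player character.
; CompleteObjective marks the current objective done, reveals the next, refreshes the UI, starts a BP_WaveManager wave with its enemy count and returns its music phase.
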(event EventBeginPlay)

(event Collision|EventActorBeginOverlap
  (params (OtherActor :type Actor%20Object%20Reference)))

(event EventTick
  (params (DeltaSeconds :type Float%20%28single-precision%29)))

(fn ConstructionScript)

(fn SetMainMenuRef
  (params (MainMenu :type W%20Main%20Object%20Reference)))

(fn StartQuest
  (bind _output_get (Variables|Default|SetObjectives (Variables|Default|GetObjectives)))
  (Utilities|Array|Add _output_get (Utilities|Struct|MakeST_Objectives "Find the Gate" false true))
  (Utilities|Array|Add _output_get (Utilities|Struct|MakeST_Objectives "Enter the Gate" false true))
  (Variables|Default|SetCurrentIndex 0)
  (bind _asbp_third_person_character (Utilities|Casting|CastToBP_ThirdPersonCharacter (Game|GetPlayerCharacter 0)))
  (Default|RefreshObjectives (Variables|/Game/ThirdPerson/Blueprints/BP_ThirdPersonCharacter.BP_ThirdPersonCharacter_C|GetMainUIRef _asbp_third_person_character))
  (Variables|Default|SetbStartedQuest true))

(fn CompleteObjective
  (bind _objectives (Variables|Default|GetObjectives))
  (bind _objectives_2 (Variables|Default|GetObjectives))
  (bind _currentindex (Variables|Default|GetCurrentIndex))
  (bind _currentindex_2 (Variables|Default|GetCurrentIndex))
  (bind _output (Utilities|Array|Get(acopy) _objectives_2 _currentindex))
  (bind _output_2 (Utilities|Array|Get(acopy) _objectives _currentindex_2))
  (bind (_text _bcompleted _visible _enemies _musicphase) (Utilities|Struct|BreakST_Objectives _output))
  (bind (_text_2 _bcompleted_2 _visible_2 _enemies_2 _musicphase_2) (Utilities|Struct|BreakST_Objectives _output_2))
  (Utilities|Array|SetArrayElem (Variables|Default|GetObjectives) (Variables|Default|GetCurrentIndex) (Utilities|Struct|MakeST_Objectives _text_2 true true _enemies_2 _musicphase_2))
  (Math|Integer|IncrementInt (Variables|Default|GetCurrentIndex)
    (:%20%20
      (Utilities|Array|SetArrayElem (Variables|Default|GetObjectives) (Variables|Default|GetCurrentIndex) (Utilities|Struct|MakeST_Objectives _text false true _enemies _musicphase))
      (bind _asbp_third_person_character (Utilities|Casting|CastToBP_ThirdPersonCharacter (Game|GetPlayerCharacter 0)))
      (Default|RefreshObjectives (Variables|/Game/ThirdPerson/Blueprints/BP_ThirdPersonCharacter.BP_ThirdPersonCharacter_C|GetMainUIRef _asbp_third_person_character))
      (bind _outactors (Actor|GetAllActorsOfClass "/Game/EnemyWaves/BP_WaveManager.BP_WaveManager_C"))
      (Default|StartWave _outactors _enemies)
      (return _musicphase))))

(fn StartQuestKillEnemies
  (bind _output_get (Variables|Default|SetObjectives (Variables|Default|GetObjectives)))
  (Utilities|Array|Add _output_get (Utilities|Struct|MakeST_Objectives "Kill All Enemies" false true 5 "NewEnumerator2"))
  (Utilities|Array|Add _output_get (Utilities|Struct|MakeST_Objectives "Kill More Enemies!" false false 8 "NewEnumerator3"))
  (Variables|Default|SetCurrentIndex 0)
  (bind _asbp_third_person_character (Utilities|Casting|CastToBP_ThirdPersonCharacter (Game|GetPlayerCharacter 0)))
  (Default|RefreshObjectives (Variables|/Game/ThirdPerson/Blueprints/BP_ThirdPersonCharacter.BP_ThirdPersonCharacter_C|GetMainUIRef _asbp_third_person_character))
  (Variables|Default|SetbStartedQuest true))