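; AC_CutsceneHandler is a cutscene component that runs the game's first cutscene through a StartFirstCutscene event.
; The event plays the passed cutscene's sequence player, stops it after a fixed delay, then fades the camera in from opaque with audio while jazz music fades up.
; It then has the third-person player character show a timed line of Onyx's dialogue, with all timing driven by hardcoded delays.
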(event Custom|StartFirstCutscene
  (params (CutScene :type Level%20Sequence%20Actor%20Object%20Reference))
  (bind _sequenceplayer (Variables|/Script/LevelSequence.LevelSequenceActor|GetSequencePlayer CutScene))
  (Sequencer|Player|Play _sequenceplayer :!class /Script/MovieScene.MovieSceneSequencePlayer)
  (Utilities|FlowControl|Delay 3.0)
  (Sequencer|Player|Stop _sequenceplayer :!class /Script/MovieScene.MovieSceneSequencePlayer)
  (CameraFades|StartCameraFade :self (Game|GetPlayerCameraManager 0) :FromAlpha 1.0 :Duration 1.0 :bShouldFadeAudio true)
  (bind _returnvalue (Audio|SpawnSound2D "/Game/Music/Jazz1.Jazz1" 1.0 1.0 0.0 0))
  (Audio|Components|Audio|FadeIn _returnvalue 2.0 1.0 0.0 "Linear" :!class /Script/Engine.AudioComponent)
  (bind _asbp_third_person_character (Utilities|Casting|CastToBP_ThirdPersonCharacter (Game|GetPlayerCharacter 0)))
  (Default|SpawnDialogue _asbp_third_person_character "Onyx:" "He said he would be here...")
  (Utilities|FlowControl|Delay 3.0)
  (Default|RemoveDialogue _asbp_third_person_character))

(event EventBeginPlay)

(event EventTick
  (params (DeltaSeconds :type Float%20%28single-precision%29)))