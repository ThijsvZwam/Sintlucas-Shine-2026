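; Melee enemy for a wave-based combat game that roams randomly until pawn sensing spots a pawn.
; It then speeds up, chases the player with AIMoveTo, plays an attack montage and directly reduces player health if within range.
; TakeDamage updates an overhead health bar, hidden until first hit.
; On death it destroys itself, triggers the player's lock-on retarget and kill time dilation, and notifies the wave manager.
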(event OnSeePawn(PawnSensing)
  (params (Pawn :type Pawn%20Object%20Reference))
  (Variables|Default|SetIsSeeingPlayer true)
  (CallFunction|FollowPlayer))

(event Custom|FollowPlayer
  (bind _returnvalue (Game|GetPlayerCharacter 0))
  (Variables|/Script/Engine.CharacterMovementComponent|SetMaxWalkSpeed (Variables|Character|GetCharacterMovement) 2.5e+02)
  (Variables|Default|SetCanAttack? true)
  (if (Variables|Default|GetIsSeeingPlayer)
    (AI|AIMoveTo self "0, 0, 0" (Game|GetPlayerCharacter 0) 5.0 false
      (:OnSuccess
        (if (Variables|Default|GetCanAttack?)
          (Utilities|FlowControl|Delay 1.0)
          (Variables|Default|SetCanAttack? false)
          (Animation|PlayAnimMontage "/Game/Characters/Mannequins/Anims/Unarmed/Attack/MM_Attack_01_Montage.MM_Attack_01_Montage" 1.0 "None")
          (if (< (Transformation|GetDistanceTo _returnvalue self) 2.5e+02)
            (bind _asbp_third_person_character (Utilities|Casting|CastToBP_ThirdPersonCharacter _returnvalue))
            (Variables|/Game/ThirdPerson/Blueprints/BP_ThirdPersonCharacter.BP_ThirdPersonCharacter_C|SetHealth _asbp_third_person_character (- (Variables|/Game/ThirdPerson/Blueprints/BP_ThirdPersonCharacter.BP_ThirdPersonCharacter_C|GetHealth _asbp_third_person_character) 10)))
          (Utilities|FlowControl|Delay 2.0)
          (Variables|Default|SetCanAttack? true))))
    (else
      (Variables|Default|SetIsSeeingPlayer false)
      (CallFunction|Roam))))

(event Custom|Roam
  (Variables|/Script/Engine.CharacterMovementComponent|SetMaxWalkSpeed (Variables|Character|GetCharacterMovement) 1.5e+02)
  (AI|AIMoveTo self (.RandomLocation (AI|Navigation|GetRandomReachablePointinRadius (Transformation|GetActorLocation self) 2.5e+03 0 0)) 0 5.0 false
    (:OnSuccess
      (CallFunction|Roam))))

(event EventBeginPlay
  (Variables|Default|SetCurrentHealth (Variables|Default|GetMaxHealth))
  (Rendering|SetVisibility (Variables|Default|GetHealth) false false)
  (CallFunction|Roam))

(event Collision|EventActorBeginOverlap
  (params (OtherActor :type Actor%20Object%20Reference)))

(event EventTick
  (params (DeltaSeconds :type Float%20%28single-precision%29)))

(fn ConstructionScript)

(fn TakeDamage
  (params (DamageAmount :type Float%20%28double-precision%29))
  (bind _output_get (Variables|Default|SetCurrentHealth (- (Variables|Default|GetCurrentHealth) DamageAmount)))
  (Rendering|SetVisibility (Variables|Default|GetHealth) true false)
  (bind _aswbp_health_bar_enemy (Utilities|Casting|CastToWBP_HealthBarEnemy (UserInterface|GetUserWidgetObject (Variables|Default|GetHealth))))
  (Default|UpdateHealthEnemy _aswbp_health_bar_enemy (Math|Float|Truncate _output_get) (Math|Float|Truncate (Variables|Default|GetMaxHealth)))
  (if (<= (Variables|Default|GetCurrentHealth) 0.0)
    (bind _outactors (Actor|GetAllActorsOfClass "BP_Enemy_C"))
    (Utilities|Array|RemoveItem _outactors self)
    (Actor|DestroyActor)
    (bind _asbp_third_person_character (Utilities|Casting|CastToBP_ThirdPersonCharacter (Game|GetPlayerCharacter 0)))
    (Default|FindNewLock _asbp_third_person_character)
    (Development|PrintString "enemy died lol")
    (bind _asbp_third_person_character_2 (Utilities|Casting|CastToBP_ThirdPersonCharacter (Game|GetPlayerCharacter 0)))
    (Default|TimeDilationKill _asbp_third_person_character_2)
    (bind _outactors_2 (Actor|GetAllActorsOfClass "/Game/EnemyWaves/BP_WaveManager.BP_WaveManager_C"))
    (Default|EnemyKilled _outactors_2)
    (bind _asaic_enemy (Utilities|Casting|CastToAIC_Enemy (Pawn|GetController)))
    (AI|Logic|StopLogic (Variables|/Script/AIModule.AIController|GetBrainComponent _asaic_enemy) "")))